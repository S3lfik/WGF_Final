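; Game mode for a timed orb-collection game that ends when the orb goal is reached or the countdown expires.
; Each wave reads a DT_WavesScenario row and spawns pickups with staggered lifetimes at random free BP_Distributors.
; Pickup destruction events award time for collections and start the next wave once none remain.
; Tick dispatches time milestones, and game over clears pickups, saves up to three record scores and shows WBP_GameOver.
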(event `self.ReceiveBeginPlay`
  (bind _outactors (`GameplayStatics.GetAllActorsOfClass` "/Game/Blueprints/BP_Distributor.BP_Distributor_C"))
  (set `self.Distributors` _outactors)
  (set `self.Lives` 3)
  (bind _returnvalue (`|CreateWidget` "/Game/UI/WBP_MainUI.WBP_MainUI_C"))
  (bind _output_get (set `self.MainUI` _returnvalue))
  (`UserWidget.AddToViewport` _output_get 0)
  (`self.SetActiveCamera`)
  (bind _output_get_2 (set `self.GameOverTimer` 25.0))
  (bind _output_get_3 (set `self.TimeRemaining` _output_get_2))
  (`/Game/UI/WBP_MainUI.InitData` (`self.MainUI`) _output_get_3 (`self.OrbsGoal`))
  (`KismetSystemLibrary.K2_SetTimerDelegate` (delegate `GameStart`) 1.0))

(event `GameStart`
  (`self.SetActorTickEnabled` true)
  (`self.StartWave`)
  (`/Game/UI/WBP_MainUI.UpdateData` (`self.MainUI`) (`self.TimeRemaining`) 0))

(event `self.ReceiveTick`
  (params (DeltaSeconds :type "Float (single-precision)"))
  (`self.UpdateRemainingTime` DeltaSeconds))

(event `StartWave`
  (bind _spawnedpickups (`self.SpawnWave`))
  (set `self.NumPickupsPendingDestroy` (`KismetArrayLibrary.Array_Length` _spawnedpickups))
  (for _array_element _spawnedpickups
    (add `/Game/Blueprints/BP_Pickup.OnPickupDestroyed` _array_element (delegate `OnPickupDestroyed_Event`))))

(event `OnPickupDestroyed_Event`
  (params (NewParam :type "/Game/Blueprints/Data/EReasonToDestroy Enum" :default "NewEnumerator0"))
  (switch `/Game/Blueprints/Data/EReasonToDestroy` NewParam
    (:`NewEnumerator0`
      (`self.PickupTimedOut`))
    (:`NewEnumerator1`
      (`self.PickupGrabbed`)))
  (bind _result (`/Engine/EditorBlueprintResources/StandardMacros.DecrementInt` (`self.NumPickupsPendingDestroy`))
    (:`  `
      (`KismetSystemLibrary.PrintString` (`KismetStringLibrary.Concat_StrStr` "Pickups left: " (`KismetStringLibrary.Conv_IntToString` _result)))
      (`self.UpdateWaveState`))))

(event `UpdateWaveState`
  (if (not (`self.IsGameOver`))
    (if (`self.Is Wave Over`)
      (`/Engine/EditorBlueprintResources/StandardMacros.IncrementInt` (`self.CurrentWaveIndex`)
        (:`  `
          (`self.StartWave`))))))

(event `GameOver`
  (params (Reason :type "/Game/Blueprints/Data/EReasonGameOver Enum" :default "NewEnumerator0"))
  (`self.HandleGameOver` Reason))

(fn `GetWaveInfo`
  (params (WaveIdx :type Integer))
  (returns (WaveInfo :type "/Game/Blueprints/Data/SWaveInfo Structure") (Found :type Boolean))
  ;[1 1 1] Get New Wave info by index
  (bind _returnvalue (`|GetDataTableRow` "/Game/Blueprints/Data/DT_WavesScenario.DT_WavesScenario" (`KismetSystemLibrary.MakeLiteralName` (`KismetStringLibrary.Conv_StringToName` (`KismetStringLibrary.Conv_IntToString` WaveIdx))))
    (:`then`
      (return _returnvalue true))
    (:`RowNotFound`
      (return (struct) false))))

(fn `HandleGameOver`
  (params (Reason :type "/Game/Blueprints/Data/EReasonGameOver Enum" :default "NewEnumerator0"))
  (set `self.IsGameOver` true)
  (`|ExecutionSequence`
    (:`then_0`
      (`self.UpdateScores`))
    (:`then_1`
      (`self.SetActorTickEnabled` false)
      (bind _outactors (`GameplayStatics.GetAllActorsOfClass` "/Script/WGF_Final.PickupBase"))
      (for _array_element _outactors
        (`self.K2_DestroyActor` _array_element)
        (`Controller.UnPossess` (`GameplayStatics.GetPlayerController` 0))
        (`Widget.RemoveFromParent` (`self.MainUI`))))
    (:`then_2`
      (bind _returnvalue (`|CreateWidget` "/Game/UI/WBP_GameOver.WBP_GameOver_C"))
      (set `/Game/UI/WBP_GameOver.Scores` (`self.Scores`) _returnvalue)
      (set `/Game/UI/WBP_GameOver.GameOverReason` Reason _returnvalue)
      (`UserWidget.AddToViewport` _returnvalue 0))))

(fn `Is Wave Over`
  (returns (bWaveOver :type Boolean))
  ;[1 1 1] If no Pickups are peding being destroyed, the wave is considered over
  (`KismetSystemLibrary.PrintString` "WaveOverCheck")
  (return (== (`self.NumPickupsPendingDestroy`) 0)))

(fn `LoadScores`
  (returns (NewParam :type "Array of /Game/Blueprints/Data/SScore Structure"))
  (bind _returnvalue (`GameplayStatics.DoesSaveGameExist` "PB_SaveGame"))
  (if _returnvalue
    (bind _returnvalue_2 (`GameplayStatics.LoadGameFromSlot` "PB_SaveGame"))
    (bind _aspb_save_game (cast `/Game/Blueprints/PB_SaveGame` _returnvalue_2))
    (return (`/Game/Blueprints/PB_SaveGame.Scores` _aspb_save_game))))

(fn `PickupGrabbed`
  (bind (_currentwaveinfo_rowname _currentwaveinfo_index _currentwaveinfo_standscount _currentwaveinfo_timestep _currentwaveinfo_timereward) (break `/Game/Blueprints/Data/SWaveInfo` (`self.CurrentWaveInfo`)))
  (set `self.TimeRemaining` (+ (`self.TimeRemaining`) _currentwaveinfo_timereward))
  (`/Engine/EditorBlueprintResources/StandardMacros.IncrementInt` (`self.OrbsCollected`)
    (:`  `
      (`/Game/UI/WBP_MainUI.UpdateData` (`self.MainUI`) (`self.TimeRemaining`) (`self.OrbsCollected`))
      (if (== (`self.OrbsGoal`) (`self.OrbsCollected`))
        (`self.GameOver` "NewEnumerator1")))))

(fn `PickupTimedOut`
  ;[1 1 1] Do nothing for now.
  (`KismetSystemLibrary.PrintString` "Event OnDestroyed"))

(fn `RestartLevel`
  (bind _returnvalue (`GameplayStatics.GetCurrentLevelName` true))
  (`GameplayStatics.OpenLevel` (`KismetStringLibrary.Conv_StringToName` _returnvalue)))

(fn `SetActiveCamera`
  (bind _outactors (`GameplayStatics.GetAllActorsOfClassWithTag` "/Script/Engine.CameraActor" "MainCamera"))
  (for _array_element _outactors
    (if (`ActorComponent.IsActive` (`CameraActor.CameraComponent` _array_element))
      (set `self.ActiveCamera` _array_element))))

(fn `SpawnWave`
  (returns (SpawnedPickups :type "Array of /Game/Blueprints/BP_Pickup Object Reference"))
  (locals (LocalPickupLifeTime :type "Float (double-precision)" :default 1.0) (LocalSpawnedPickups :type "Array of /Game/Blueprints/BP_Pickup Object Reference"))
  (bind _currentwaveindex (`self.CurrentWaveIndex`))
  (bind (_currentwaveinfo_rowname _currentwaveinfo_index _currentwaveinfo_standscount) (break `/Game/Blueprints/Data/SWaveInfo` (`self.CurrentWaveInfo`)))
  (bind (_currentwaveinfo_rowname_2 _currentwaveinfo_index_2 _currentwaveinfo_standscount_2 _currentwaveinfo_timestep) (break `/Game/Blueprints/Data/SWaveInfo` (`self.CurrentWaveInfo`)))
  (bind (_currentwaveinfo_rowname_3 _currentwaveinfo_index_3 _currentwaveinfo_standscount_3 _currentwaveinfo_timestep_2) (break `/Game/Blueprints/Data/SWaveInfo` (`self.CurrentWaveInfo`)))
  (`|ExecutionSequence`
    (:`then_0`
      ;[1 1 1] Get Current wave info
      (bind (_waveinfo _found) (`self.GetWaveInfo` _currentwaveindex))
      (if _found
        (set `self.CurrentWaveInfo` _waveinfo))
      (`KismetSystemLibrary.PrintString` (`KismetStringLibrary.Concat_StrStr` "Wave: " (`KismetStringLibrary.Conv_IntToString` _currentwaveindex)))
      (for _array_element (`self.Distributors`)
        (`/Game/Blueprints/BP_Distributor.Reset` _array_element)
        (set `local.LocalPickupLifeTime` _currentwaveinfo_timestep)))
    (:`then_1`
      ;[1 1 1] Spawn Pickups
      (for _ (range 1 (+ _currentwaveinfo_standscount 1))
        (bind _returnvalue (`/Game/Blueprints/BP_Distributor.SpawnPickup` (`self.GetRandomFreeDistributor` (`self.Distributors`)) (`local.LocalPickupLifeTime`)))
        (bind _asbp_pickup (cast `/Game/Blueprints/BP_Pickup` _returnvalue)) ; Remove when/if the code is moved to C++
        (`KismetArrayLibrary.Array_Add` (`local.LocalSpawnedPickups`) _asbp_pickup)
        (set `local.LocalPickupLifeTime` (+ (`local.LocalPickupLifeTime`) _currentwaveinfo_timestep_2))))
    (:`then_2`
      ;[1 1 1] Return Spawned Pickups for binding
      (return (`local.LocalSpawnedPickups`)))))

(fn `UpdateLevelVisuals`
  (bind _returnvalue (`KismetMathLibrary.FTrunc` (/ (`self.TimeRemaining`) 5.0)))
  (if (<= _returnvalue 3)
    (`self.TimeMilestoneDispatch` (- 3 _returnvalue))))

(fn `UpdateRemainingTime`
  (params (DeltaTime :type "Float (double-precision)"))
  (bind _output_get (set `self.TimeRemaining` (- (`self.TimeRemaining`) DeltaTime)))
  (if (<= _output_get 0.0)
    (`self.GameOver` "NewEnumerator0")
    (else
      (`self.UpdateLevelVisuals`))))

(fn `UpdateScores`
  (locals (LocalScores :type "Array of /Game/Blueprints/Data/SScore Structure") (ScoresSet :type "Set of /Game/Blueprints/Data/SScore Structure"))
  (bind _scores (`self.Scores`))
  (bind _output_score (break `/Game/Blueprints/Data/SScore` (`|GetArrayItem` (`self.Scores`))))
  (bind _newparam (`self.LoadScores`))
  (set `self.Scores` _newparam)
  ;[1 1 1] IsNotEmpty
  (if (> (`KismetArrayLibrary.Array_Length` (`self.Scores`)) 0)
    ;[1 1 1] IfNewRecord
    (if (< _output_score (`self.Score`))
      (`KismetArrayLibrary.Array_Insert` (`self.Scores`) (make `/Game/Blueprints/Data/SScore` (`self.Score`) (`KismetMathLibrary.Now`)))
      (if (> (`KismetArrayLibrary.Array_Length` _scores) 3)
        (`KismetArrayLibrary.Array_Resize` _scores 3))
      ;[1 1 1] Rewrite
      (bind _returnvalue (`GameplayStatics.CreateSaveGameObject` "/Game/Blueprints/PB_SaveGame.PB_SaveGame_C" :!label _label))
      (set `/Game/Blueprints/PB_SaveGame.Scores` (`self.Scores`) _returnvalue)
      (`GameplayStatics.SaveGameToSlot` _returnvalue "PB_SaveGame"))
    (else
      ;[1 1 1] PopulateEmptyArray
      (if (> (`self.Score`) 0)
        (`KismetArrayLibrary.Array_Add` (`self.Scores`) (make `/Game/Blueprints/Data/SScore` (`self.Score`) (`KismetMathLibrary.Now`)))
        (goto _label)))))

(fn `UserConstructionScript`)