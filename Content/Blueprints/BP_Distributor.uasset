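; BP_Distributor is a stand that spawns and holds one BP_Pickup at a time.
; SpawnPickup refuses while occupied; otherwise it spawns a pickup at the Arrow's transform, passes the given time as its DestroyTime and returns it.
; Tick polls the stored pickup reference and frees the stand once that pickup is no longer valid.
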(event `self.ReceiveBeginPlay`
  (set `self.isOccupied` false))

(event `self.ReceiveTick`
  (params (DeltaSeconds :type "Float (single-precision)"))
  (`self.UpdateIsOccupied`))

(fn `SpawnPickup`
  (params (Time :type "Float (double-precision)"))
  (returns (Output_Get :type "/Game/Blueprints/BP_Pickup Object Reference"))
  (if (`self.isOccupied`)
    (`KismetSystemLibrary.PrintString` "An attempt to use an occupied Stand")
    (else
      (bind _returnvalue (`|SpawnActorFromClass` "/Game/Blueprints/BP_Pickup.BP_Pickup_C" (`SceneComponent.K2_GetComponentToWorld` (`self.Arrow`)) "AlwaysSpawn" "OverrideRootScale" null null))
      (`/Engine/EditorBlueprintResources/StandardMacros.IsValid` _returnvalue
        (:`Is Valid`
          (bind _output_get (set `self.SpawnedPickup` _returnvalue))
          (set `/Game/Blueprints/BP_Pickup.DestroyTime` Time _output_get)
          (set `self.isOccupied` true)
          (return _output_get))
        (:`Is Not Valid`
          (`KismetSystemLibrary.PrintString` "Hello"))))))

(fn `UpdateIsOccupied`
  (if (`self.isOccupied`)
    (`/Engine/EditorBlueprintResources/StandardMacros.IsValid` (`self.SpawnedPickup`)
      (:`Is Not Valid`
        (set `self.isOccupied` false)
        (`KismetSystemLibrary.PrintString` "Occupation Switched")))))

(fn `UserConstructionScript`)